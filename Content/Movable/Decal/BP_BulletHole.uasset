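; BP_BulletHole is a bullet hole decal actor that fades and removes itself shortly after spawning.
; BeginPlay creates a dynamic instance of BulletHole_Mat, assigns it to the decal and sets a short life span.
; Tick lowers CurAlpha by a fixed step and writes it to the Opacity parameter, so fade speed depends on frame rate.
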(event `self.ReceiveBeginPlay`
  (bind _returnvalue (`KismetMaterialLibrary.CreateDynamicMaterialInstance` "/Game/Movable/Decal/bulletHole_Mat.bulletHole_Mat"))
  (bind _output_get (set `self.decalMat` _returnvalue))
  (`DecalComponent.SetDecalMaterial` (`self.Decal`) _output_get)
  (`self.SetLifeSpan` 3.0))

(event `self.ReceiveTick`
  (params (DeltaSeconds :type "Float (single-precision)"))
  (set `self.curAlpha` (- (`self.curAlpha`) 0.004))
  (`MaterialInstanceDynamic.SetScalarParameterValue` (`self.decalMat`) "Opacity" (`self.curAlpha`)))

(fn `UserConstructionScript`)