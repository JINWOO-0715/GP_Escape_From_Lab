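; BP_SpawnWeapon is a weapon spawn point that creates one random rifle when play begins.
; On BeginPlay it spawns a BP_WeaponBase at its own location, adjusting for collision or skipping the spawn if still blocked.
; A random roll through a chain of branches picks one of four hard-coded weapon names and passes it to SetupWeapon on the new actor.
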(event `self.ReceiveBeginPlay`
  (bind _returnvalue (`|SpawnActorFromClass` "/Game/Movable/WeaponBP/BP_WeaponBase.BP_WeaponBase_C" (`KismetMathLibrary.Conv_VectorToTransform` (`self.K2_GetActorLocation`)) "AdjustIfPossibleButDontSpawnIfColliding" "OverrideRootScale" null null))
  (bind _output_get (set `self.random` (`KismetMathLibrary.RandomInteger` 4)))
  (if (== _output_get 0)
    (`WeaponBase.SetupWeapon` _returnvalue "AR4")
    (elif (== _output_get 1)
      (`WeaponBase.SetupWeapon` _returnvalue "AK74")
      (elif (== _output_get 2)
        (`WeaponBase.SetupWeapon` _returnvalue "KAVAL")
        (elif (== _output_get 3)
          (`WeaponBase.SetupWeapon` _returnvalue "AK47"))))))

(fn `UserConstructionScript`)