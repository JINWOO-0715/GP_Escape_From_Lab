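; BP_Item is an item actor whose mesh switches to a red-outlined variant to highlight it for the player's Swat character.
; Every Tick, it checks the character's CollisionItemon flag and its own CollisionSwat flag.
; When both are true, it applies RedOutlineItemMesh from its DefaultItemName row in ItemDataTable.
; Otherwise it applies the row's normal ItemMesh and clears CollisionSwat, so highlighting relies on mesh swapping.
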(event `self.ReceiveTick`
  (params (DeltaSeconds :type "Float (single-precision)"))
  (bind _asswat (cast `Swat` (`GameplayStatics.GetPlayerCharacter` 0)))
  (if (`Swat.collisionItemon` _asswat)
    (if (`self.collisionSwat`)
      (bind _returnvalue (`|GetDataTableRow` (`self.ItemDataTable`) (`self.DefaultItemName`))
        (:`then`
          (`StaticMeshComponent.SetStaticMesh` (`self.MeshComp`) (`.RedOutlineItemMesh` (break `ItemData` _returnvalue)))))
      (else
        (bind _returnvalue_2 (`|GetDataTableRow` (`self.ItemDataTable`) (`self.DefaultItemName`) :!label _label)
          (:`then`
            (`StaticMeshComponent.SetStaticMesh` (`self.MeshComp`) (`.ItemMesh` (break `ItemData` _returnvalue_2)))
            (set `self.collisionSwat` false)))))
    (else
      (goto _label))))

(fn `UserConstructionScript`)