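; BP_WeaponBase is a weapon actor that shows a red-outline highlight through mesh swapping, based on collision state with the player's Swat character.
; Every Tick it checks Swat's CollisionWeapon and its own IsCollisionSwat, then sets RedOutlineMesh or WeaponStaticMesh from the DefaultWeaponName row of WeaponDataTable.
; Restoring the normal mesh clears IsCollisionSwat, which this graph never sets true.
; RedOutline and WhiteOutline are empty, unused events.
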(event `RedOutline`)

(event `self.ReceiveTick`
  (params (DeltaSeconds :type "Float (single-precision)"))
  (bind _asswat (cast `Swat` (`GameplayStatics.GetPlayerCharacter` 0)))
  (if (`Swat.collisionWeapon` _asswat)
    (if (`self.isCollisionSwat`)
      (bind _returnvalue (`|GetDataTableRow` (`self.WeaponDataTable`) (`self.DefaultWeaponName`))
        (:`then`
          (`StaticMeshComponent.SetStaticMesh` (`self.StaticMeshComp`) (`.RedOutlineMesh` (break `WeaponData` _returnvalue)))))
      (else
        (bind _returnvalue_2 (`|GetDataTableRow` (`self.WeaponDataTable`) (`self.DefaultWeaponName`) :!label _label)
          (:`then`
            (`StaticMeshComponent.SetStaticMesh` (`self.StaticMeshComp`) (`.WeaponStaticMesh` (break `WeaponData` _returnvalue_2)))
            (set `self.isCollisionSwat` false)))))
    (else
      (goto _label))))

(event `WhiteOutline`)

(fn `UserConstructionScript`)