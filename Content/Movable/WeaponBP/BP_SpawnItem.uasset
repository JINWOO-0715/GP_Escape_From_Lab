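; Item spawner actor that places one random pickup at its own location when play begins.
; BeginPlay rolls one of three indices and passes it to SpawnItemReq, which spawns a BP_Item with collision-adjusted placement.
; The index selects an ammo, SevenAmmo or medkit row name, which SetupItemFromDT uses to configure the item before its mesh starts simulating physics.
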(event `self.ReceiveBeginPlay`
  (bind _output_get (set `self.random` (`KismetMathLibrary.RandomInteger` 3)))
  (`self.SpawnItemReq` _output_get))

(event `SpawnItemReq`
  (params (NewParam :type Integer))
  (bind _returnvalue (`|SpawnActorFromClass` "/Game/Movable/WeaponBP/BP_Item.BP_Item_C" (`KismetMathLibrary.Conv_VectorToTransform` (`self.K2_GetActorLocation`)) "AdjustIfPossibleButDontSpawnIfColliding" "OverrideRootScale" null null))
  (if (== NewParam 0)
    (bind _output_get (set `Pickups.DefaultItemName` "Ammo" _returnvalue))
    (`Pickups.SetupItemFromDT` _returnvalue _output_get)
    (`PrimitiveComponent.SetSimulatePhysics` (`Pickups.MeshComp` _returnvalue) true :!label _label)
    (elif (== NewParam 1)
      (bind _output_get_2 (set `Pickups.DefaultItemName` "SevenAmmo" _returnvalue))
      (`Pickups.SetupItemFromDT` _returnvalue _output_get_2)
      (goto _label)
      (elif (== NewParam 2)
        (bind _output_get_3 (set `Pickups.DefaultItemName` "Medkit" _returnvalue))
        (`Pickups.SetupItemFromDT` _returnvalue _output_get_3)
        (goto _label)))))

(fn `UserConstructionScript`)