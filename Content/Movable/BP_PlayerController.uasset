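; Player controller Blueprint that shows a loading screen on network clients while the current level is Transition_Map.
; On BeginPlay, only without authority, it creates a BP_LoadingWidget, adds it to the viewport and keeps it hidden.
; Tick, also remote-only, polls the current level name every frame and toggles the widget's visibility to match.
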(event `self.ReceiveBeginPlay`
  (`/Engine/EditorBlueprintResources/ActorMacros.Switch Has Authority`
    (:`Remote`
      (bind _returnvalue (`|CreateWidget` "/Game/Movable/UI/BP_LoadingWidget.BP_LoadingWidget_C" (`GameplayStatics.GetPlayerController` 0)))
      (`/Engine/EditorBlueprintResources/StandardMacros.IsValid` _returnvalue
        (:`Is Valid`
          (bind _output_get (set `self.LoadingWidget` _returnvalue))
          (`UserWidget.AddToViewport` _output_get 0)
          (`Widget.SetVisibility` _output_get "Hidden"))))))

(event `self.ReceiveTick`
  (params (DeltaSeconds :type "Float (single-precision)"))
  (bind _loadingwidget (`self.LoadingWidget`))
  (`/Engine/EditorBlueprintResources/ActorMacros.Switch Has Authority`
    (:`Remote`
      (bind _returnvalue (`GameplayStatics.GetCurrentLevelName` true))
      (if (`KismetStringLibrary.EqualEqual_StrStr` _returnvalue "Transition_Map")
        (`/Engine/EditorBlueprintResources/StandardMacros.IsValid` _loadingwidget
          (:`Is Valid`
            (`Widget.SetVisibility` _loadingwidget "Visible")))
        (else
          (`/Engine/EditorBlueprintResources/StandardMacros.IsValid` _loadingwidget
            (:`Is Valid`
              (`Widget.SetVisibility` _loadingwidget "Hidden"))))))))

(fn `UserConstructionScript`)