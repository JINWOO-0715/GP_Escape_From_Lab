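; Player controller for the Title map that shows the title menu and handles the move into gameplay.
; On BeginPlay outside dedicated servers, it creates BP_TitleWidget on the Title level with UI-only input and a visible cursor.
; With authority, Tick polls the title game mode and, while exactly two players are present, calls a multicast-named event that sets IsButtonEnabled.
; A separate event asks the game mode to server travel, named for Stage 1.
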(event `setIsButtonEnabledTrueMultCast`
  (set `self.isButtonEnabled` true))

(event `serverTravelToStage1`
  (bind _asbp_title_game_mode (cast `/Game/Movable/Maps/Title/BP_TitleGameMode` (`GameplayStatics.GetGameMode`)))
  (`/Game/Movable/Maps/Title/BP_TitleGameMode.serverTravel` _asbp_title_game_mode))

(event `self.ReceiveBeginPlay`
  (bind _returnvalue (`GameplayStatics.GetCurrentLevelName` true))
  (if (`KismetStringLibrary.EqualEqual_StrStr` _returnvalue "Title")
    (if (not (`KismetSystemLibrary.IsDedicatedServer`))
      (bind _returnvalue_2 (`|CreateWidget` "/Game/Movable/Maps/Title/BP_TitleWidget.BP_TitleWidget_C" self))
      (bind _output_get (set `self.widget` _returnvalue_2))
      (`UserWidget.AddToViewport` _output_get 0)
      (`WidgetBlueprintLibrary.SetInputMode_UIOnlyEx` self _output_get)
      (set `self.bShowMouseCursor` true))))

(event `self.ReceiveTick`
  (params (DeltaSeconds :type "Float (single-precision)"))
  (`/Engine/EditorBlueprintResources/ActorMacros.Switch Has Authority`
    (:`Authority`
      (bind _asbp_title_game_mode (cast `/Game/Movable/Maps/Title/BP_TitleGameMode` (`GameplayStatics.GetGameMode`)))
      (if (== (`/Game/Movable/Maps/Title/BP_TitleGameMode.curPlayerNum` _asbp_title_game_mode) 2)
        (`self.setIsButtonEnabledTrueMultCast`)))))

(fn `UserConstructionScript`)