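; BP_Stage1Light is a light actor that periodically flickers its bulb material and rect light together.
; BeginPlay creates a dynamic material on the Light component and picks a random delay of a few seconds, fixed per instance.
; Tick runs through that Delay to replay the BulbFlickering timeline, whose curve drives both the LightIntensity material parameter and the scaled RectLight intensity.
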(event `self.ReceiveBeginPlay`
  (bind _returnvalue (`PrimitiveComponent.CreateDynamicMaterialInstance` (`self.light`) 0 "/Game/Industrial_Office_02/Materials/M_Lights_c_d.M_Lights_c_d" "None"))
  (set `self.bulbIntensity` _returnvalue)
  (set `self.RandomDuration` (`KismetMathLibrary.RandomFloatInRange` 3.0 6.0)))

(event `self.ReceiveTick`
  (params (DeltaSeconds :type "Float (single-precision)"))
  (`KismetSystemLibrary.Delay` (`self.RandomDuration`))
  (`self.flickering`))

(event `flickering`
  (bind (_direction _bulbintensity) (`Timeline|bulbFlickering` :!via `PlayFromStart`)
    (:`Update`
      (`MaterialInstanceDynamic.SetScalarParameterValue` (`self.bulbIntensity`) "LightIntensity" _bulbintensity)
      (`LightComponent.SetIntensity` (`self.RectLight`) (* 5000 _bulbintensity)))))

(fn `UserConstructionScript`)