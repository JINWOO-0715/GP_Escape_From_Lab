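; BP_DestructibleWood is a wooden prop that breaks apart when it takes damage.
; Any damage, regardless of amount, runs applyDamage, which deals a large fixed hit to the Destructible component along its forward vector and fires a RadialForce impulse.
; The same event swaps visuals by revealing the Destructible, hiding the intact StaticMesh and disabling that mesh's collision.
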(event `applyDamage`
  (bind _destructible (`self.Destructible`))
  (bind _staticmesh (`self.StaticMesh`))
  (`DestructibleComponent.ApplyDamage` _destructible 1000.0 (`SceneComponent.K2_GetComponentLocation` _destructible) (`SceneComponent.GetForwardVector` _destructible) 0.0)
  (`RadialForceComponent.FireImpulse` (`self.RadialForce`))
  (`SceneComponent.SetVisibility` (`self.Destructible`) true false)
  (`SceneComponent.SetVisibility` _staticmesh false false)
  (`PrimitiveComponent.SetCollisionEnabled` _staticmesh "NoCollision"))

(event `self.ReceiveAnyDamage`
  (params (Damage :type "Float (single-precision)") (DamageType :type "DamageType Object Reference") (InstigatedBy :type "Controller Object Reference") (DamageCauser :type "Actor Object Reference"))
  (`self.applyDamage`))

(fn `UserConstructionScript`)