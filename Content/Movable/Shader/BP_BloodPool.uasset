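; BP_BloodPool is a blood pool actor that repeatedly plays randomly chosen sounds from three audio sources.
; Tick runs into a 0.8-second Delay, which throttles playback to roughly that interval.
; Each branch rolls its own random integer, so Audio1, Audio2 and Audio3 have decreasing odds and some cycles play nothing.
; BeginPlay, overlap and construction logic are empty.
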(event `self.ReceiveTick`
  (params (DeltaSeconds :type "Float (single-precision)"))
  (bind _returnvalue (`KismetMathLibrary.RandomIntegerInRange` 0 2))
  (`KismetSystemLibrary.Delay` 0.8)
  (if (== _returnvalue 0)
    (`AudioComponent.Play` (`self.Audio1`) 0.0)
    (elif (== _returnvalue 1)
      (`AudioComponent.Play` (`self.Audio2`) 0.0)
      (elif (== _returnvalue 2)
        (`AudioComponent.Play` (`self.Audio3`) 0.0)))))

(fn `UserConstructionScript`)