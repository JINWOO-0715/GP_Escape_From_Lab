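; Stage 3 female zombie character that sets itself up from data and plays an attack animation.
; On BeginPlay it turns off its Box collision, loads mesh, HP, speed and attack power from the "Female" row of DT_ZombieDataTable, and binds Attack to the FemaleAttack event.
; AnyDamage only disables box and capsule collision when HP is below one, without subtracting HP here, and the Box overlap handler is empty.
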(event `self.ReceiveBeginPlay`
  (`PrimitiveComponent.SetCollisionEnabled` (`self.Box`) "NoCollision")
  (`self.InitZombie`)
  (add `self.FemaleAttack` (delegate `Attack`)))

(event `Attack`
  (`self.PlayAnimMontage` "/Game/Movable/Zombie/Anim/FemaleAttack_Montage.FemaleAttack_Montage"))

(event `InitZombie`
  (bind _returnvalue (`|GetDataTableRow` "/Game/Movable/Zombie/DT_ZombieDataTable.DT_ZombieDataTable" "Female")
    (:`then`
      (`SkeletalMeshComponent.SetAnimInstanceClass` (`self.Mesh`) "/Game/Movable/Zombie/Anim/Stage3FemaleAnim_BP.Stage3FemaleAnim_BP_C")
      (bind (_zombiename _zombiemesh _zombiehp _zombiespeed _zombieattackpower) (break `ZombieData` _returnvalue))
      (`SkinnedMeshComponent.SetSkinnedAssetAndUpdate` (`self.Mesh`) _zombiemesh true)
      (set `self.hp` _zombiehp)
      (bind _output_get (set `self.speed` _zombiespeed))
      (set `self.attackPower` _zombieattackpower)
      (set `CharacterMovementComponent.MaxWalkSpeed` _output_get (`self.CharacterMovement`)))))

(event `self.Box.OnComponentBeginOverlap`
  (params (OverlappedComponent :type "PrimitiveComponent Object Reference") (OtherActor :type "Actor Object Reference") (OtherComp :type "PrimitiveComponent Object Reference") (OtherBodyIndex :type Integer) (bFromSweep :type Boolean) (SweepResult :type "HitResult Structure (by ref)")))

(event `self.ReceiveAnyDamage`
  (params (Damage :type "Float (single-precision)") (DamageType :type "DamageType Object Reference") (InstigatedBy :type "Controller Object Reference") (DamageCauser :type "Actor Object Reference"))
  (if (< (`self.hp`) 1.0)
    (`PrimitiveComponent.SetCollisionEnabled` (`self.Box`) "NoCollision")
    (`PrimitiveComponent.SetCollisionEnabled` (`self.CapsuleComponent`) "NoCollision")))

(fn `UserConstructionScript`)