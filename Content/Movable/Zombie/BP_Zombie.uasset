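; BP_Zombie is a networked zombie enemy with Female, Male, Security and LittleGirl variants.
; Setup applies data-table stats, mesh and animation class, and creates dissolve materials for all variants but LittleGirl.
; Tick polls HP: the server updates counts, drops random items plus a KeyCard every third kill, then destroys the actor, while clients animate the dissolve.
; Overlaps with MySwat set proximity flags.
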(event `SetRandomRead`
  (set `self.SaveRandom` (`KismetMathLibrary.RandomInteger` 3)))

(event `SetupZombieReq`
  (params (ZombieName :type Name))
  (bind _returnvalue (`|GetDataTableRow` "/Game/Movable/Zombie/DT_ZombieDataTable.DT_ZombieDataTable" ZombieName)
    (:`then`
      (bind (_zombiename _zombiemesh _zombiehp _zombiespeed _zombieattackpower) (break `ZombieData` _returnvalue))
      (if (`KismetStringLibrary.EqualEqual_StrStr` _zombiename "Female")
        (`SkeletalMeshComponent.SetAnimInstanceClass` (`self.Mesh`) "/Game/Movable/AnimationBP/Zombie/AnimBP_Female.AnimBP_Female_C")
        (`SkinnedMeshComponent.SetSkinnedAssetAndUpdate` (`self.Mesh`) _zombiemesh true :!label _label)
        (set `self.hp` _zombiehp)
        (bind _output_get (set `self.speed` _zombiespeed))
        (set `self.attackPower` _zombieattackpower)
        (set `CharacterMovementComponent.MaxWalkSpeed` _output_get (`self.CharacterMovement`))
        (set `self.WayNum` (`self.SaveRandom`))
        (set `self.InitLocation` (`self.K2_GetActorLocation`))
        (elif (`KismetStringLibrary.EqualEqual_StrStr` _zombiename "Male")
          (`SkeletalMeshComponent.SetAnimInstanceClass` (`self.Mesh`) "/Game/Movable/AnimationBP/Zombie/AnimBP_MaleZombie.AnimBP_MaleZombie_C")
          (goto _label)
          (elif (`KismetStringLibrary.EqualEqual_StrStr` _zombiename "Security")
            (`SkeletalMeshComponent.SetAnimInstanceClass` (`self.Mesh`) "/Game/Movable/AnimationBP/Zombie/AnimBP_Security.AnimBP_Security_C")
            (goto _label)
            (elif (`KismetStringLibrary.EqualEqual_StrStr` _zombiename "LittleGirl")
              (`SkeletalMeshComponent.SetAnimInstanceClass` (`self.Mesh`) "/Game/Movable/AnimationBP/Zombie/AnimBP_LittleGirlZombie.AnimBP_LittleGirlZombie_C")
              (goto _label))))))))

(event `self.ReceiveTick`
  (params (DeltaSeconds :type "Float (single-precision)"))
  (bind _zombiemanager (`self.Zombiemanager`))
  (bind _parameter_value (`self.Parameter Value`))
  (bind _returnvalue (- (`self.Parameter Value`) (+ DeltaSeconds 0.02)))
  (`/Engine/EditorBlueprintResources/ActorMacros.Switch Has Authority`
    (:`Authority`
      (if (<= (`self.hp`) 0.0)
        (`KismetSystemLibrary.Delay` 4.0)
        (`/Engine/EditorBlueprintResources/StandardMacros.IsValid` _zombiemanager
          (:`Is Valid`
            (`/Engine/EditorBlueprintResources/StandardMacros.DecrementInt` (`/Game/Movable/Zombie/BP_ZombieManager.ZombieCount` _zombiemanager)
              (:`  `
                (if (`KismetMathLibrary.RandomBoolWithWeight` 0.2)
                  (`|SpawnActorFromClass` "/Game/Movable/WeaponBP/BP_SpawnItem.BP_SpawnItem_C" (`self.GetTransform`) "Undefined" "OverrideRootScale" null null))
                (bind _asmy_game_mode (cast `MyGameMode` (`GameplayStatics.GetGameMode`)))
                (bind _deathzombie (`MyGameMode.deathZombie` _asmy_game_mode))
                (`/Engine/EditorBlueprintResources/StandardMacros.IncrementInt` _deathzombie
                  (:`  `
                    (if (== (mod _deathzombie 3) 0)
                      (bind _returnvalue_2 (`|SpawnActorFromClass` "/Game/Movable/WeaponBP/BP_Item.BP_Item_C" (`self.GetTransform`) "AdjustIfPossibleButAlwaysSpawn" "OverrideRootScale" null null))
                      (set `Pickups.DefaultItemName` "KeyCard" _returnvalue_2))
                    (`KismetSystemLibrary.PrintString` "zombieBye" true true (struct :`G` 0.66 :`B` 1.0 :`A` 1.0) 10.0)
                    (`self.K2_DestroyActor`)))))))))
    (:`Remote`
      (if (<= (`self.hp`) 0.0)
        (if (`self.isDead`)
          (if (`self.canDissolve`)
            (`MaterialInstanceDynamic.SetScalarParameterValue` (`self.mat1`) "dissolve" _parameter_value)
            (`MaterialInstanceDynamic.SetScalarParameterValue` (`self.mat2`) "dissolve" _parameter_value)
            (`/Engine/EditorBlueprintResources/StandardMacros.IsValid` (`self.mat3`)
              (:`Is Valid`
                (`MaterialInstanceDynamic.SetScalarParameterValue` (`self.mat3`) "dissolve" _returnvalue)
                (`MaterialInstanceDynamic.SetScalarParameterValue` (`self.mat4`) "dissolve" _returnvalue)
                (`MaterialInstanceDynamic.SetScalarParameterValue` (`self.mat5`) "dissolve" _returnvalue)
                (`MaterialInstanceDynamic.SetScalarParameterValue` (`self.mat6`) "dissolve" _returnvalue))
              (:`Is Not Valid`
                _))
            (set `self.Parameter Value` _returnvalue))
          (else
            (set `self.isDead` true)
            (`KismetSystemLibrary.Delay` 2.0)
            (set `self.canDissolve` true)))))))

(event `self.ReceiveActorBeginOverlap`
  (params (OtherActor :type "Actor Object Reference"))
  (cast `/Game/Movable/MySwat` OtherActor)
  (set `self.isOverlapped` true))

(event `self.ReceiveActorEndOverlap`
  (params (OtherActor :type "Actor Object Reference"))
  (cast `/Game/Movable/MySwat` OtherActor)
  (set `self.isOverlapped` false))

(event `self.Box.OnComponentBeginOverlap`
  (params (OverlappedComponent :type "PrimitiveComponent Object Reference") (OtherActor :type "Actor Object Reference") (OtherComp :type "PrimitiveComponent Object Reference") (OtherBodyIndex :type Integer) (bFromSweep :type Boolean) (SweepResult :type "HitResult Structure (by ref)"))
  (bind (_returnvalue_roll _returnvalue_pitch) (`KismetMathLibrary.BreakRotator` (`self.K2_GetActorRotation`)))
  (`/Engine/EditorBlueprintResources/ActorMacros.Switch Has Authority`
    (:`Authority`
      (bind _asmy_swat (cast `/Game/Movable/MySwat` OtherActor))
      (set `self.IsColliedBox` true)
      (`/Engine/EditorBlueprintResources/ActorMacros.Switch Has Authority`
        (:`Remote`
          (bind (_returnvalue_roll_2 _returnvalue_pitch_2 _returnvalue_yaw) (`KismetMathLibrary.BreakRotator` (`KismetMathLibrary.FindLookAtRotation` (`self.K2_GetActorLocation`) (`self.K2_GetActorLocation` _asmy_swat))))
          (`self.K2_SetActorRotation` (`KismetMathLibrary.MakeRotator` _returnvalue_roll_2 _returnvalue_pitch _returnvalue_yaw)))))))

(event `self.ReceiveBeginPlay`
  (`self.SetRandomRead`)
  (`self.SetupZombieReq` "None")
  (`self.zombieMatReq`))

(event `zombieMatReq`
  (`self.SetZombieMatReq`))

(event `SetZombieMatReq`
  (switch `name` (`self.DefaultZombieName`)
    (:`Security`
      (bind _returnvalue (`KismetMaterialLibrary.CreateDynamicMaterialInstance` "/Game/StarterContent/Materials/M_Metal_Burnished_Steel.M_Metal_Burnished_Steel"))
      (set `self.mat1` _returnvalue)
      (bind _returnvalue_2 (`KismetMaterialLibrary.CreateDynamicMaterialInstance` "/Game/NonMovable/Zombie/SKMesh/Security/Face_Police_Zombie_MAT.Face_Police_Zombie_MAT"))
      (set `self.mat2` _returnvalue_2)
      (`PrimitiveComponent.SetMaterial` (`self.Mesh`) 0 (`self.mat1`))
      (`PrimitiveComponent.SetMaterial` (`self.Mesh`) 1 (`self.mat2`)))
    (:`Male`
      (bind _returnvalue_3 (`KismetMaterialLibrary.CreateDynamicMaterialInstance` "/Game/NonMovable/Zombie/SKMesh/Male/Ch10_body.Ch10_body"))
      (set `self.mat1` _returnvalue_3)
      (bind _returnvalue_4 (`KismetMaterialLibrary.CreateDynamicMaterialInstance` "/Game/NonMovable/Zombie/SKMesh/Male/Ch10_body1.Ch10_body1"))
      (set `self.mat2` _returnvalue_4)
      (`PrimitiveComponent.SetMaterial` (`self.Mesh`) 0 (`self.mat1`))
      (`PrimitiveComponent.SetMaterial` (`self.Mesh`) 1 (`self.mat2`)))
    (:`Female`
      (bind _returnvalue_5 (`KismetMaterialLibrary.CreateDynamicMaterialInstance` "/Game/NonMovable/Zombie/SKMesh/FemaleResearcher/Jill_HiMidRes_Hair_MAT.Jill_HiMidRes_Hair_MAT"))
      (set `self.mat1` _returnvalue_5)
      (bind _returnvalue_6 (`KismetMaterialLibrary.CreateDynamicMaterialInstance` "/Game/NonMovable/Zombie/SKMesh/FemaleResearcher/Jill_HiMidRes_EyeSpec_MAT.Jill_HiMidRes_EyeSpec_MAT"))
      (set `self.mat2` _returnvalue_6)
      (bind _returnvalue_7 (`KismetMaterialLibrary.CreateDynamicMaterialInstance` "/Game/NonMovable/Zombie/SKMesh/FemaleResearcher/Jill_HiMidRes_Eyes_MAT.Jill_HiMidRes_Eyes_MAT"))
      (set `self.mat3` _returnvalue_7)
      (bind _returnvalue_8 (`KismetMaterialLibrary.CreateDynamicMaterialInstance` "/Game/NonMovable/Zombie/SKMesh/FemaleResearcher/Jill_HiMidRes_Teeth_MAT.Jill_HiMidRes_Teeth_MAT"))
      (set `self.mat4` _returnvalue_8)
      (bind _returnvalue_9 (`KismetMaterialLibrary.CreateDynamicMaterialInstance` "/Game/NonMovable/Zombie/SKMesh/FemaleResearcher/Jill_HiMidRes_Body_MAT.Jill_HiMidRes_Body_MAT"))
      (set `self.mat5` _returnvalue_9)
      (bind _returnvalue_10 (`KismetMaterialLibrary.CreateDynamicMaterialInstance` "/Game/NonMovable/Zombie/SKMesh/FemaleResearcher/Jill_HiMidRes_Gown_MAT.Jill_HiMidRes_Gown_MAT"))
      (set `self.mat6` _returnvalue_10)
      (`PrimitiveComponent.SetMaterial` (`self.Mesh`) 0 (`self.mat1`))
      (`PrimitiveComponent.SetMaterial` (`self.Mesh`) 1 (`self.mat2`))
      (`PrimitiveComponent.SetMaterial` (`self.Mesh`) 2 (`self.mat3`))
      (`PrimitiveComponent.SetMaterial` (`self.Mesh`) 3 (`self.mat4`))
      (`PrimitiveComponent.SetMaterial` (`self.Mesh`) 4 (`self.mat5`))
      (`PrimitiveComponent.SetMaterial` (`self.Mesh`) 5 (`self.mat6`)))))

(event `self.Box.OnComponentEndOverlap`
  (params (OverlappedComponent :type "PrimitiveComponent Object Reference") (OtherActor :type "Actor Object Reference") (OtherComp :type "PrimitiveComponent Object Reference") (OtherBodyIndex :type Integer))
  (`/Engine/EditorBlueprintResources/ActorMacros.Switch Has Authority`
    (:`Authority`
      (cast `/Game/Movable/MySwat` OtherActor)
      (set `self.IsColliedBox` false))))

(fn `NewFunction_0`)

(fn `UserConstructionScript`)