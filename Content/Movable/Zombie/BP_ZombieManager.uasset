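; BP_ZombieManager is a spawner actor that creates a small batch of BP_Zombie characters when play begins.
; BeginPlay requests the spawn event, which creates each zombie at the manager's location, adjusting for collisions but always spawning.
; Each zombie gets the default "Male" name and its default controller.
; A short Delay loops the event back until ZombieCount reaches its fixed cap, staggering the spawns.
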(event `self.ReceiveBeginPlay`
  (`self.SpawnZombie_Req`))

(event `SpawnZombie_Req`
  (bind _zombiecount (`self.ZombieCount`))
  (bind _returnvalue (`|SpawnActorFromClass` "/Game/Movable/Zombie/BP_Zombie.BP_Zombie_C" (`KismetMathLibrary.Conv_VectorToTransform` (`self.K2_GetActorLocation` self)) "AdjustIfPossibleButAlwaysSpawn" "OverrideRootScale" null null :!label _label))
  (set `Zombie.DefaultZombieName` "Male" _returnvalue)
  (`Pawn.SpawnDefaultController` _returnvalue)
  (`KismetSystemLibrary.Delay` 0.1)
  (`/Engine/EditorBlueprintResources/StandardMacros.IncrementInt` _zombiecount
    (:`  `
      (if (not (>= _zombiecount 5))
        (goto _label)))))

(fn `UserConstructionScript`)